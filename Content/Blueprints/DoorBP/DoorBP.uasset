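; Door actor Blueprint that the player opens and closes with the E key while standing in its trigger box.
; Overlapping the box enables input for player controller 0, and leaving it disables input again.
; Each E press prints a debug string and flip-flops a timeline between play and reverse, whose track drives the door mesh's relative yaw while keeping pitch and roll.
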(event `self.Box.OnComponentBeginOverlap`
  (params (OverlappedComponent :type "PrimitiveComponent Object Reference") (OtherActor :type "Actor Object Reference") (OtherComp :type "PrimitiveComponent Object Reference") (OtherBodyIndex :type Integer) (bFromSweep :type Boolean) (SweepResult :type "HitResult Structure (by ref)"))
  (`self.EnableInput` (`GameplayStatics.GetPlayerController` 0)))

(event `self.Box.OnComponentEndOverlap`
  (params (OverlappedComponent :type "PrimitiveComponent Object Reference") (OtherActor :type "Actor Object Reference") (OtherComp :type "PrimitiveComponent Object Reference") (OtherBodyIndex :type Integer))
  (`self.DisableInput` (`GameplayStatics.GetPlayerController` 0)))

(event `Key|E`
  (params (Key :type "Key Structure"))
  (bind _doorsm (`self.DoorSM`))
  (bind (_relativerotation_roll _relativerotation_pitch) (`KismetMathLibrary.BreakRotator` (`SceneComponent.RelativeRotation` _doorsm)))
  (:`Pressed`
    (`KismetSystemLibrary.PrintString` "Test Successful!")
    (`/Engine/EditorBlueprintResources/StandardMacros.FlipFlop`
      (:`A`
        (bind (_direction _doormovementtrack) (`Timeline|DoorMovementTL` :!label _label)
          (:`Update`
            (`SceneComponent.K2_SetRelativeRotation` _doorsm (`KismetMathLibrary.MakeRotator` _relativerotation_roll _relativerotation_pitch _doormovementtrack) false false))))
      (:`B`
        (goto _label :!via `Reverse`)))))

(fn `UserConstructionScript`)